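; Code-entry puzzle object that builds a random answer on the server at BeginPlay and calls CorrectCode when the entered code matches.
; The answer is made by shuffling and concatenating a set of number strings.
; DoOnce gates control evaluation of full-length input and the start of a timeout timer.
; A wrong code or an expired timer resets the lamps and clears the timer on the server.
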(event `self.ReceiveBeginPlay`
  (bind _m_randomnumbersstring (`self.M_RandomNumbersString`))
  (`/Engine/EditorBlueprintResources/ActorMacros.Switch Has Authority`
    (:`Authority`
      (add `self.M_ResetPuzzle` (`|CreateDelegate` :!event `ResetDoOnce1`))
      (`KismetArrayLibrary.Array_Shuffle` _m_randomnumbersstring)
      (for _index (range (`KismetArrayLibrary.Array_Length` _m_randomnumbersstring))
        (set `self.M_CorrectCode` (`KismetStringLibrary.Concat_StrStr` (`self.M_CorrectCode`) (`|GetArrayItem` _m_randomnumbersstring _index)))))))

(event `ResetDoOnce2`
  (goto _label :!via `Reset`))

(event `self.CheckInput`
  (`|ExecutionSequence`
    (:`then_0`
      (if (== (`KismetStringLibrary.Len` (`self.M_InputCode`)) (`KismetStringLibrary.Len` (`self.M_CorrectCode`)))
        (`/Engine/EditorBlueprintResources/StandardMacros.DoOnce` false :!label _label
          (:`Completed`
            (if (`KismetStringLibrary.EqualEqual_StrStr` (`self.M_InputCode`) (`self.M_CorrectCode`))
              (`self.CorrectCode`)
              (`KismetSystemLibrary.PrintString` "Correct Code")
              (else
                (`/Engine/EditorBlueprintResources/ActorMacros.Switch Has Authority`
                  (:`Authority`
                    (`self.ResetLamps`)
                    (`KismetSystemLibrary.K2_ClearAndInvalidateTimerHandle` (`self.ResetTimer`))
                    (`KismetSystemLibrary.PrintString` "incorrect Code")))))))))
    (:`then_1`
      (`/Engine/EditorBlueprintResources/StandardMacros.DoOnce` false :!label _label_2
        (:`Completed`
          (`KismetSystemLibrary.PrintString` "TimerStarted")
          (bind _returnvalue (`KismetSystemLibrary.K2_SetTimerDelegate` (delegate `CallReset`) 35.0))
          (set `self.ResetTimer` _returnvalue))))))

(event `ResetDoOnce1`
  (`self.ResetDoOnce2`)
  (`KismetSystemLibrary.Delay` 0.4)
  (goto _label_2 :!via `Reset`))

(event `CallReset`
  (`/Engine/EditorBlueprintResources/ActorMacros.Switch Has Authority`
    (:`Authority`
      (`self.ResetLamps`)
      (`KismetSystemLibrary.K2_ClearAndInvalidateTimerHandle` (`self.ResetTimer`)))))

(fn `UserConstructionScript`)