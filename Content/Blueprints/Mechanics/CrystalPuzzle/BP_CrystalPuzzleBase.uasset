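; Base Blueprint for a crystal puzzle piece that drives the visuals of a laser beam.
; On BeginPlay it assigns its Niagara component to the laser VFX variable.
; Each Tick it matches the effect's world rotation to the sphere mesh and sets the "Beam End" parameter to the hit point when blocking, otherwise to the default end.
; The graph only reads the blocking flag and both endpoints, without computing them.
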(event `self.ReceiveBeginPlay`
  (set `self.M_LaserVFX` (`self.Niagara`)))

(event `UpdateBeamHitLocation`
  (`FXSystemComponent.SetVectorParameter` (`self.Niagara`) "Beam End" (`self.M_HitEnd`)))

(event `self.ReceiveTick`
  (params (DeltaSeconds :type "Float (single-precision)"))
  (`SceneComponent.K2_SetWorldRotation` (`self.Niagara`) (`SceneComponent.K2_GetComponentRotation` (`self.M_SphereMesh`)) false false)
  (if (`self.M_bIsBlocking`)
    (`self.UpdateBeamHitLocation`)
    (else
      (`self.UpdateBeamEndLocation`))))

(event `UpdateBeamEndLocation`
  (`FXSystemComponent.SetVectorParameter` (`self.Niagara`) "Beam End" (`self.M_End`)))

(fn `UserConstructionScript`)