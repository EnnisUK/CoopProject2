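; AC_Chat_PC is an actor component for player controllers that provides multiplayer text chat.
; On BeginPlay, the local controller creates the chat UI widget and keeps a reference to its chat panel.
; Enter focuses the chat, and the mouse wheel scrolls it.
; A server RPC relays each message through every PlayerArray controller's component to a client RPC, which adds it to that player's chat.
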(event `self.ReceiveBeginPlay`
  (if (`Controller.IsLocalPlayerController` (cast `PlayerController` (`self.GetOwner`) :!pure true))
    (bind _returnvalue (`|CreateWidget` "/Game/Widgets/ChatWidget/WBP_ChatUI.WBP_ChatUI_C"))
    (bind _output_get (set `self.ChatUIRef` _returnvalue))
    (`UserWidget.AddToViewport` _output_get 0)
    (set `self.WBP ChatRef` (`/Game/Widgets/ChatWidget/WBP_ChatUI.WBP_Chat` _output_get))))

(event `Key|Enter`
  (params (Key :type "Key Structure"))
  (:`Pressed`
    (`/Game/Widgets/ChatWidget/WBP_Chat.FocusChat` (`self.WBP ChatRef`))))

(event `Key|MouseScrollUp`
  (params (Key :type "Key Structure"))
  (:`Pressed`
    (`/Game/Widgets/ChatWidget/WBP_Chat.Scroll` (`self.WBP ChatRef`) true)))

(event `Key|MouseScrollDown`
  (params (Key :type "Key Structure"))
  (:`Pressed`
    (`/Game/Widgets/ChatWidget/WBP_Chat.Scroll` (`self.WBP ChatRef`) false)))

(event `ServerRPC_SendChatMessage`
  (params (Message :type String))
  (for _array_element (`GameStateBase.PlayerArray` (`GameplayStatics.GetGameState`))
    (`self.ClientRPC_AddChatMessage` (`Actor.GetComponentByClass` (`PlayerState.GetPlayerController` _array_element) "AC_Chat_PC_C") Message)))

(event `ClientRPC_AddChatMessage`
  (params (Message :type String))
  (`/Game/Widgets/ChatWidget/WBP_Chat.AddChatMessage` (`self.WBP ChatRef`) Message))