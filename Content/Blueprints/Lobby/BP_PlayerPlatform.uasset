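; Lobby player platform that offers a friend invite button and hosts the friends list at its location.
; On the server, setup finds the shared BP_FriendList actor and links the button widget back to this platform.
; ShowFriendsList moves that single list actor here and collapses the button.
; Bound invite events toggle the button; hiding also selects the default character class and closes the list if positioned here.
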(event `self.ReceiveBeginPlay`
  (set `self.As BP Lobby GM` (cast `/Game/Blueprints/Lobby/BP_LobbyGM` (`GameplayStatics.GetGameMode`) :!pure true))
  (`self.SetupServer`)
  (add `self.HideInvite` (delegate `HideInviteEvent`))
  (add `self.ShowInvite` (delegate `ShowInviteEvent`)))

(event `ShowInviteEvent`
  (`SceneComponent.SetVisibility` (`self.OpenFriendsListButton`) true false))

(event `HideInviteEvent`
  (`/Game/Blueprints/Lobby/BP_LobbyGM.SelectCharacterClassByIndex` (`self.As BP Lobby GM`) (`self.M_PC`) 0)
  (`SceneComponent.SetVisibility` (`self.OpenFriendsListButton`) false false)
  (if (== (`SceneComponent.K2_GetComponentLocation` (`self.FriendListLocation`)) (`self.K2_GetActorLocation` (`self.FriendListRef`)) :`ErrorTolerance` 5.0)
    (`/Game/Blueprints/Lobby/BP_FriendList.Show` (`self.FriendListRef`) false null)))

(fn `SetupServer`
  (if (`KismetSystemLibrary.IsServer`)
    (bind _returnvalue (`GameplayStatics.GetActorOfClass` "/Game/Blueprints/Lobby/BP_FriendList.BP_FriendList_C"))
    (set `self.FriendListRef` _returnvalue)
    (bind _aswbp_open_friends_list_button (cast `/Game/Widgets/WBP_OpenFriendsListButton` (`WidgetComponent.GetWidget` (`self.OpenFriendsListButton`))))
    (set `/Game/Widgets/WBP_OpenFriendsListButton.LobbyPlayerPlatformRef` self _aswbp_open_friends_list_button)
    (`SceneComponent.SetVisibility` (`self.OpenFriendsListButton`) true false)))

(fn `ShowFriendsList`
  (params (bShow :type Boolean))
  (bind _friendlistref (`self.FriendListRef`))
  (bind _returnvalue (`WidgetComponent.GetWidget` (`self.OpenFriendsListButton`)))
  (if bShow
    (`Widget.SetVisibility` _returnvalue "Collapsed")
    (`self.K2_SetActorLocation` _friendlistref (`SceneComponent.K2_GetComponentLocation` (`self.FriendListLocation`)) false false)
    (`/Game/Blueprints/Lobby/BP_FriendList.Show` _friendlistref true self)
    (else
      (`Widget.SetVisibility` _returnvalue "Visible"))))

(fn `UserConstructionScript`)