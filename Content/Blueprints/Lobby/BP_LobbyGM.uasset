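; Lobby game mode that shows joined players as characters on player platforms and handles kicking and server travel into the match.
; BeginPlay orders platforms by index tag; login and logout update the controller list, wait for setup via a polling macro, then fill or clear platforms.
; UpdatePlayerInfo pushes name and ready state to the platform character, sets CanStart from only the first controller's ready flag, and requests a retry if none matches.
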(event `self.ReceiveBeginPlay`
  (`self.SetupPlatforms`))

(event `self.K2_PostLogin`
  (params (NewPlayer :type "PlayerController Object Reference"))
  (`KismetArrayLibrary.Array_Add` (`self.PCs`) NewPlayer)
  (`self.PlatformsDone` :!label _label
    (:`true`
      (`self.UpdatePlayersOnPlatforms`))))

(event `self.K2_OnLogout`
  (params (ExitingController :type "Controller Object Reference"))
  (bind _asplayer_controller (cast `PlayerController` ExitingController))
  (`KismetArrayLibrary.Array_RemoveItem` (`self.PCs`) _asplayer_controller)
  (goto _label))

(fn `KickPlayer`
  (params (PlayerToKick :type "PlayerController Object Reference"))
  (`AdvancedSessionsLibrary.KickPlayer` PlayerToKick))

(fn `SetupPlatforms`
  (bind _outactors (`GameplayStatics.GetAllActorsOfClass` "/Game/Blueprints/Lobby/BP_PlayerPlatform.BP_PlayerPlatform_C"))
  (for _index (range (+ (`KismetArrayLibrary.Array_LastIndex` _outactors) 1))
    (bind _outactors_2 (`GameplayStatics.GetAllActorsOfClassWithTag` "/Game/Blueprints/Lobby/BP_PlayerPlatform.BP_PlayerPlatform_C" (`KismetStringLibrary.Conv_StringToName` (`KismetStringLibrary.Conv_IntToString` _index))))
    (`KismetArrayLibrary.Array_Add` (`self.PlayerPlatforms`) (`|GetArrayItem` _outactors_2)))
  (set `self.bPlatformsSetupComplete` true))

(fn `StartMatch`
  (if (`KismetSystemLibrary.IsServer`)
    (`AdvancedSessionsLibrary.ServerTravel` "/Game/ThirdPerson/Maps/ThirdPersonMap")
    (for _array_element (`self.PCs`)
      (bind _asbp_lobby_pc (cast `/Game/Blueprints/Lobby/BP_LobbyPC` _array_element))
      (`/Game/Blueprints/Lobby/BP_LobbyPC.OnStartMatch` _asbp_lobby_pc))))

(fn `UpdatePlayerInfo`
  (params (RequestPC :type "PlayerController Object Reference"))
  (bind _requestpc (`local.RequestPC`))
  (bind _asbp_lobby_pc (cast `/Game/Blueprints/Lobby/BP_LobbyPC` (`local.RequestPC`) :!pure true))
  (bind (_playerlobbyinfopc_pc _playerlobbyinfopc_playername _playerlobbyinfopc_bready) (break `/Game/Blueprints/Lobby/S_PlayerLobbyInfo` (`/Game/Blueprints/Lobby/BP_LobbyPC.PlayerLobbyInfoPC` _asbp_lobby_pc)))
  (`/Engine/EditorBlueprintResources/StandardMacros.IsValid` RequestPC
    (:`Is Valid`
      (for _array_element (`self.PlayerPlatforms`)
        (if (== (`PlayerPlatform.M_PC` _array_element) RequestPC)
          (bind _asbp_main_character (cast `/Game/Blueprints/Characters/BP_MainCharacter` (`PlayerPlatform.M_CurrentCharacter` _array_element))
            (:`then`
              (`/Game/Blueprints/Characters/BP_MainCharacter.UpdatePlayerLobbyInfo` _asbp_main_character (make `/Game/Blueprints/Lobby/S_PlayerLobbyInfo` (`local.RequestPC`) (`KismetTextLibrary.Conv_StringToText` (`AdvancedSessionsLibrary.GetPlayerName` _requestpc)) _playerlobbyinfopc_bready (`Controller.PlayerState` _requestpc)))
              (for _array_element_2 (`self.PCs`)
                (bind _asbp_lobby_pc_2 (cast `/Game/Blueprints/Lobby/BP_LobbyPC` _array_element_2))
                (bind (_playerlobbyinfopc_pc_2 _playerlobbyinfopc_playername_2 _playerlobbyinfopc_bready_2) (break `/Game/Blueprints/Lobby/S_PlayerLobbyInfo` (`/Game/Blueprints/Lobby/BP_LobbyPC.PlayerLobbyInfoPC` _asbp_lobby_pc_2)))
                (if (== _playerlobbyinfopc_bready_2 true)
                  (set `self.bCanStart` true)
                  (else
                    (set `self.bCanStart` false)))
                (return)))
            (:`CastFailed`
              (`KismetSystemLibrary.PrintString` "Cast Failed")))))
      (`/Game/Blueprints/Lobby/BP_LobbyPC.TryAgainUpdatingLobbyInfo` _asbp_lobby_pc))))

(fn `UpdatePlayersOnPlatforms`
  (locals (Loop_PCAlreadyAdded :type Boolean))
  (for _array_element (`self.PCs`)
    (set `local.Loop_PCAlreadyAdded` false)
    (for _array_element_2 (`self.PlayerPlatforms`)
      (if (== (`PlayerPlatform.M_PC` _array_element_2) _array_element)
        (set `local.Loop_PCAlreadyAdded` true)
        (break)))
    (if (not (`local.Loop_PCAlreadyAdded`))
      (for _array_element_3 (`self.PlayerPlatforms`)
        (`/Engine/EditorBlueprintResources/StandardMacros.IsValid` (`PlayerPlatform.M_PC` _array_element_3)
          (:`Is Not Valid`
            (`PlayerPlatform.SpawnCharacter` _array_element_3 _array_element)
            (break))))))
  (for _array_element_4 (`self.PlayerPlatforms`)
    (if (not (`KismetArrayLibrary.Array_Contains` (`self.PCs`) (`PlayerPlatform.M_PC` _array_element_4)))
      (`PlayerPlatform.Clear` _array_element_4))))

(fn `UserConstructionScript`)