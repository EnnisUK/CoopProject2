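; Lobby player controller that handles a player's ready state, character choice and lobby UI.
; On BeginPlay the local controller creates the lobby widget and binds its ready button, while server-side controllers without UI report to BP_LobbyGM after a short delay.
; R toggles readiness through the game mode, and a looping MultiGate alternates between two character classes.
; Match start shows a loading screen and disables input.
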(event `self.ReceiveBeginPlay`
  (bind _lobbyuiref (`self.LobbyUiRef`))
  (set `self.LobbyGMRef` (cast `/Game/Blueprints/Lobby/BP_LobbyGM` (`GameplayStatics.GetGameMode`) :!pure true))
  (`self.Setup`)
  (`/Engine/EditorBlueprintResources/StandardMacros.IsValid` _lobbyuiref
    (:`Is Valid`
      (add `Button.OnClicked` (`/Game/Widgets/Modular/WBP_Button.Button_55` (`/Game/Widgets/WBP_LobbyUI.B_Ready` _lobbyuiref)) (`|CreateDelegate` :!event `ToggleReadyOnServer`)))
    (:`Is Not Valid`
      (`/Engine/EditorBlueprintResources/ActorMacros.Switch Has Authority`
        (:`Authority`
          (`self.TryAgainUpdatingLobbyInfo`))))))

(event `TryAgainUpdatingLobbyInfo`
  (`KismetSystemLibrary.Delay` 0.1)
  (bind _asbp_lobby_gm (cast `/Game/Blueprints/Lobby/BP_LobbyGM` (`GameplayStatics.GetGameMode`)))
  (`/Game/Blueprints/Lobby/BP_LobbyGM.UpdatePlayerInfo` _asbp_lobby_gm self))

(event `ToggleReadyOnServer`
  (bind _playerlobbyinfopc (`self.PlayerLobbyInfoPC`))
  (setmembers `/Game/Blueprints/Lobby/S_PlayerLobbyInfo` :`StructRef` _playerlobbyinfopc :`bReady` (not (`.bReady_8_EDD8FBDA47FD05D56ED0F88456EEC7C8` (break `/Game/Blueprints/Lobby/S_PlayerLobbyInfo` _playerlobbyinfopc))))
  (bind _asbp_lobby_gm (cast `/Game/Blueprints/Lobby/BP_LobbyGM` (`GameplayStatics.GetGameMode`)))
  (`/Game/Blueprints/Lobby/BP_LobbyGM.UpdatePlayerInfo` _asbp_lobby_gm self))

(event `Key|R`
  (params (Key :type "Key Structure"))
  (:`Pressed`
    (`self.ToggleReadyOnServer`)))

(event `OnStartMatch`
  (`/Game/Widgets/WBP_LobbyUI.ShowLoadingScreen` (`self.LobbyUiRef`))
  (`self.DisableInput` self))

(event `SelectCharOnServer`
  (bind _lobbygmref (`self.LobbyGMRef`))
  (`|MultiGate` false true 1
    (:`Out 0`
      (`/Game/Blueprints/Lobby/BP_LobbyGM.SelectCharacterClassByIndex` _lobbygmref self 0))
    (:`Out 1`
      (`/Game/Blueprints/Lobby/BP_LobbyGM.SelectCharacterClassByIndex` _lobbygmref self 1))))

(fn `Setup`
  (if (`self.IsLocalPlayerController`)
    (set `self.bShowMouseCursor` true)
    (`WidgetBlueprintLibrary.SetInputMode_GameAndUIEx` self null "DoNotLock" false)
    (bind _returnvalue (`|CreateWidget` "/Game/Widgets/WBP_LobbyUI.WBP_LobbyUI_C"))
    (bind _output_get (set `self.LobbyUiRef` _returnvalue))
    (`UserWidget.AddToViewport` _output_get 0)))

(fn `UserConstructionScript`)