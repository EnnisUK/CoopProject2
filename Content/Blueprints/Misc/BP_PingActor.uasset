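; BP_PingActor is a short-lived ping marker that shows a coloured WBP_Ping widget and destroys itself two seconds after spawning.
; After a brief BeginPlay delay, the server calls ClientRPC_ChangeColour and starts the destroy timer.
; That event picks one of two colours based on whether a valid owner has authority.
; The Colour RepNotify applies the result to the widget's ping image.
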(event `self.ReceiveBeginPlay`
  (`KismetSystemLibrary.Delay` 0.02)
  (bind _aswbp_ping (cast `/Game/Widgets/WBP_Ping` (`WidgetComponent.GetWidget` (`self.Widget`))))
  (set `self.As WBP Ping` _aswbp_ping)
  (bind _asbp_main_character (cast `/Game/Blueprints/Characters/BP_MainCharacter` (`GameplayStatics.GetPlayerCharacter` 0)))
  (set `self.As BP Main Character` _asbp_main_character)
  (if (`KismetSystemLibrary.IsServer`)
    (`self.ClientRPC_ChangeColour`)
    (`KismetSystemLibrary.K2_SetTimerDelegate` (delegate `DestroySelf`) 2.0)))

(event `DestroySelf`
  (`self.K2_DestroyActor`))

(event `ClientRPC_ChangeColour`
  (bind _returnvalue (`self.GetOwner`))
  (`/Engine/EditorBlueprintResources/StandardMacros.IsValid` _returnvalue
    (:`Is Valid`
      (if (`self.HasAuthority` _returnvalue)
        (set `self.Colour` (struct :`R` 0.266062 :`B` 1.0 :`A` 1.0))
        (else
          (set `self.Colour` (struct :`R` 1.0 :`G` 0.202119 :`A` 1.0) :!label _label))))
    (:`Is Not Valid`
      (goto _label))))

(fn `OnRep_Colour`
  (bind _aswbp_ping (cast `/Game/Widgets/WBP_Ping` (`WidgetComponent.GetWidget` (`self.Widget`))))
  (`Image.SetColorAndOpacity` (`/Game/Widgets/WBP_Ping.PingImage` _aswbp_ping) (`self.Colour`)))

(fn `UserConstructionScript`)