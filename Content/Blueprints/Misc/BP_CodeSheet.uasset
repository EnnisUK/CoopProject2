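; Code sheet actor that displays the lamp puzzle's correct code as up to eight coloured entries on a WBP_LampColourCode widget.
; On BeginPlay the server polls until all players are ready, then links the widget to MTA and triggers the colouring.
; Each digit of MTA.MCorrectCode maps to an MTA colour, stored in per-slot variables whose OnRep functions repaint the widget on clients.
; SetVisFunction toggles the widget's visibility from the server.
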(event `self.ReceiveBeginPlay`
  (`/Engine/EditorBlueprintResources/ActorMacros.Switch Has Authority`
    (:`Authority`
      (bind _asbp_afgi_main_instance (cast `/Game/Blueprints/Systems/BP_AFGI_MainInstance` (`GameplayStatics.GetGameInstance`)))
      (bind _playersconnected (`/Game/Blueprints/Systems/BP_AFGI_MainInstance.ArePlayersReady` _asbp_afgi_main_instance :!label _label))
      (if _playersconnected
        (bind _aswbp_lamp_colour_code (cast `/Game/Widgets/WBP_LampColourCode` (`WidgetComponent.GetWidget` (`self.Widget`))))
        (set `self.As WBP Lamp Colour Code` _aswbp_lamp_colour_code)
        (set `/Game/Widgets/WBP_LampColourCode.CodeObjectRef` (`self.M_TA`) _aswbp_lamp_colour_code)
        (`KismetSystemLibrary.Delay` 0.5)
        (`self.CallMulticastEvent`)
        (else
          (`KismetSystemLibrary.Delay` 0.2)
          (goto _label))))))

(event `CallMulticastEvent`
  (`self.ChangeColours`))

(event `ChangeColours`
  (bind _as_wbp_lamp_colour_code (`self.As WBP Lamp Colour Code`))
  (bind _as_wbp_lamp_colour_code_2 (`self.As WBP Lamp Colour Code`))
  (bind _as_wbp_lamp_colour_code_3 (`self.As WBP Lamp Colour Code`))
  (for (_array_element _array_index) (`KismetStringLibrary.GetCharacterArrayFromString` (`CodeMovableObject.M_CorrectCode` (`self.M_TA`)))
    (switch `int` _array_index
      (:`0`
        (bind (_outputpin _output_get) (`self.CheckNumber` (`/Game/Widgets/WBP_LampColourCode.Code1` _as_wbp_lamp_colour_code_2) _array_element))
        (bind _output_get_2 (set `self.Output Get` _output_get))
        (`Image.SetColorAndOpacity` _outputpin _output_get_2))
      (:`1`
        (bind (_outputpin_2 _output_get_3) (`self.CheckNumber` (`/Game/Widgets/WBP_LampColourCode.Code2` _as_wbp_lamp_colour_code_2) _array_element))
        (bind _output_get_4 (set `self.Colour2` _output_get_3))
        (`Image.SetColorAndOpacity` _outputpin_2 _output_get_4))
      (:`2`
        (bind (_outputpin_3 _output_get_5) (`self.CheckNumber` (`/Game/Widgets/WBP_LampColourCode.Code3` _as_wbp_lamp_colour_code_3) _array_element))
        (bind _output_get_6 (set `self.Colour3` _output_get_5))
        (`Image.SetColorAndOpacity` _outputpin_3 _output_get_6))
      (:`3`
        (bind (_outputpin_4 _output_get_7) (`self.CheckNumber` (`/Game/Widgets/WBP_LampColourCode.Code4` _as_wbp_lamp_colour_code_3) _array_element))
        (bind _output_get_8 (set `self.Colour4` _output_get_7))
        (`Image.SetColorAndOpacity` _outputpin_4 _output_get_8))
      (:`4`
        (bind (_outputpin_5 _output_get_9) (`self.CheckNumber` (`/Game/Widgets/WBP_LampColourCode.Code5` _as_wbp_lamp_colour_code_3) _array_element))
        (bind _output_get_10 (set `self.Colour5` _output_get_9))
        (`Image.SetColorAndOpacity` _outputpin_5 _output_get_10))
      (:`5`
        (bind (_outputpin_6 _output_get_11) (`self.CheckNumber` (`/Game/Widgets/WBP_LampColourCode.Code6` _as_wbp_lamp_colour_code_3) _array_element))
        (bind _output_get_12 (set `self.Colour6` _output_get_11))
        (`Image.SetColorAndOpacity` _outputpin_6 _output_get_12))
      (:`6`
        (bind (_outputpin_7 _output_get_13) (`self.CheckNumber` (`/Game/Widgets/WBP_LampColourCode.Code7` _as_wbp_lamp_colour_code) _array_element))
        (bind _output_get_14 (set `self.Colour7` _output_get_13))
        (`Image.SetColorAndOpacity` _outputpin_7 _output_get_14))
      (:`7`
        (bind (_outputpin_8 _output_get_15) (`self.CheckNumber` (`/Game/Widgets/WBP_LampColourCode.Code8` _as_wbp_lamp_colour_code) _array_element))
        (bind _output_get_16 (set `self.Colour8` _output_get_15))
        (`Image.SetColorAndOpacity` _outputpin_8 _output_get_16)))))

(event `ChangeVis`
  (bind _widget (`self.Widget`))
  (if (`SceneComponent.bHiddenInGame` _widget)
    (`SceneComponent.SetHiddenInGame` _widget false false)
    (else
      (`SceneComponent.SetHiddenInGame` _widget true false))))

(event `GlobalFunctionsInterface.SetVisFunction`
  (`/Engine/EditorBlueprintResources/ActorMacros.Switch Has Authority`
    (:`Authority`
      (`self.ChangeVis`))))

(fn `CheckNumber`
  (params (Target :type "Image Object Reference") (Array :type String))
  (returns (OutputPin :type "Image Object Reference") (Output_Get :type "LinearColor Structure"))
  (bind _m_ta (`self.M_TA`))
  (bind _m_ta_2 (`self.M_TA`))
  (bind _m_ta_3 (`self.M_TA`))
  (if (`KismetStringLibrary.EqualEqual_StrStr` Array "1")
    (return Target (`CodeMovableObject.M_Colour1` _m_ta_2))
    (elif (`KismetStringLibrary.EqualEqual_StrStr` Array "2")
      (return Target (`CodeMovableObject.M_Colour2` _m_ta_2))
      (elif (`KismetStringLibrary.EqualEqual_StrStr` Array "3")
        (return Target (`CodeMovableObject.M_Colour3` _m_ta_3))
        (elif (`KismetStringLibrary.EqualEqual_StrStr` Array "4")
          (return Target (`CodeMovableObject.M_Colour4` _m_ta_3))
          (elif (`KismetStringLibrary.EqualEqual_StrStr` Array "5")
            (return Target (`CodeMovableObject.M_Colour5` _m_ta))
            (elif (`KismetStringLibrary.EqualEqual_StrStr` Array "6")
              (return Target (`CodeMovableObject.M_Colour6` _m_ta))
              (elif (`KismetStringLibrary.EqualEqual_StrStr` Array "7")
                (return Target (`CodeMovableObject.M_Colour7` _m_ta))
                (elif (`KismetStringLibrary.EqualEqual_StrStr` Array "8")
                  (return Target (`CodeMovableObject.M_Colour8` _m_ta)))))))))))

(fn `OnRep_Colour2`
  (bind _aswbp_lamp_colour_code (cast `/Game/Widgets/WBP_LampColourCode` (`WidgetComponent.GetWidget` (`self.Widget`))))
  (bind _output_get (set `self.As WBP Lamp Colour Code` _aswbp_lamp_colour_code))
  (`Image.SetColorAndOpacity` (`/Game/Widgets/WBP_LampColourCode.Code2` _output_get) (`self.Colour2`)))

(fn `OnRep_Colour3`
  (bind _aswbp_lamp_colour_code (cast `/Game/Widgets/WBP_LampColourCode` (`WidgetComponent.GetWidget` (`self.Widget`))))
  (bind _output_get (set `self.As WBP Lamp Colour Code` _aswbp_lamp_colour_code))
  (`Image.SetColorAndOpacity` (`/Game/Widgets/WBP_LampColourCode.Code3` _output_get) (`self.Colour3`)))

(fn `OnRep_Colour4`
  (bind _aswbp_lamp_colour_code (cast `/Game/Widgets/WBP_LampColourCode` (`WidgetComponent.GetWidget` (`self.Widget`))))
  (bind _output_get (set `self.As WBP Lamp Colour Code` _aswbp_lamp_colour_code))
  (`Image.SetColorAndOpacity` (`/Game/Widgets/WBP_LampColourCode.Code4` _output_get) (`self.Colour4`)))

(fn `OnRep_Colour5`
  (bind _aswbp_lamp_colour_code (cast `/Game/Widgets/WBP_LampColourCode` (`WidgetComponent.GetWidget` (`self.Widget`))))
  (bind _output_get (set `self.As WBP Lamp Colour Code` _aswbp_lamp_colour_code))
  (`Image.SetColorAndOpacity` (`/Game/Widgets/WBP_LampColourCode.Code5` _output_get) (`self.Colour5`)))

(fn `OnRep_Colour6`
  (bind _aswbp_lamp_colour_code (cast `/Game/Widgets/WBP_LampColourCode` (`WidgetComponent.GetWidget` (`self.Widget`))))
  (bind _output_get (set `self.As WBP Lamp Colour Code` _aswbp_lamp_colour_code))
  (`Image.SetColorAndOpacity` (`/Game/Widgets/WBP_LampColourCode.Code6` _output_get) (`self.Colour6`)))

(fn `OnRep_Colour7`
  (bind _aswbp_lamp_colour_code (cast `/Game/Widgets/WBP_LampColourCode` (`WidgetComponent.GetWidget` (`self.Widget`))))
  (bind _output_get (set `self.As WBP Lamp Colour Code` _aswbp_lamp_colour_code))
  (`Image.SetColorAndOpacity` (`/Game/Widgets/WBP_LampColourCode.Code7` _output_get) (`self.Colour7`)))

(fn `OnRep_Colour8`
  (bind _aswbp_lamp_colour_code (cast `/Game/Widgets/WBP_LampColourCode` (`WidgetComponent.GetWidget` (`self.Widget`))))
  (bind _output_get (set `self.As WBP Lamp Colour Code` _aswbp_lamp_colour_code))
  (`Image.SetColorAndOpacity` (`/Game/Widgets/WBP_LampColourCode.Code8` _output_get) (`self.Colour8`)))

(fn `OnRep_Output Get`
  (bind _aswbp_lamp_colour_code (cast `/Game/Widgets/WBP_LampColourCode` (`WidgetComponent.GetWidget` (`self.Widget`))))
  (bind _output_get (set `self.As WBP Lamp Colour Code` _aswbp_lamp_colour_code))
  (`Image.SetColorAndOpacity` (`/Game/Widgets/WBP_LampColourCode.Code1` _output_get) (`self.Output Get`)))

(fn `UserConstructionScript`)