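; Game instance that handles friend session invites for a two-player game and applies the screen resolution at startup.
; Init waits briefly, then sets the resolution from MResolution through an r.setres console command.
; An accepted invite destroys the current session and joins the new one, even if destruction fails.
; InvitePlayer sends invites only from the server, and ArePlayersReady checks that exactly two PlayerController actors exist.
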(event `self.ReceiveInit`
  (bind (_m_resolution_x _m_resolution_y) (break `IntPoint` (`self.M_Resolution`)))
  (`KismetSystemLibrary.Delay` 0.2)
  (`KismetSystemLibrary.ExecuteConsoleCommand` (`KismetStringLibrary.Concat_StrStr` "r.setres " (`KismetStringLibrary.Conv_IntToString` _m_resolution_x) "x" (`KismetStringLibrary.Conv_IntToString` _m_resolution_y)) null))

(event `self.OnSessionInviteAccepted`
  (params (LocalPlayerNum :type Integer) (PersonInvited :type "BPUniqueNetId Structure") (SessionToJoin :type "BlueprintSessionResult Structure (by ref)"))
  (bind _returnvalue (`self.GetLocalController` null))
  (`DestroySessionCallbackProxy.DestroySession` _returnvalue
    (:`OnSuccess`
      _)
    (:`OnFailure`
      _))
  (`JoinSessionCallbackProxy.JoinSession` _returnvalue SessionToJoin))

(fn `ArePlayersReady`
  (returns (PlayersConnected :type Boolean))
  (bind _outactors (`GameplayStatics.GetAllActorsOfClass` "/Script/Engine.PlayerController"))
  (return (== (`KismetArrayLibrary.Array_Length` _outactors) 2)))

(fn `InvitePlayer`
  (params (FriendUniqueNetId :type "BPUniqueNetId Structure (by ref)"))
  (if (`KismetSystemLibrary.IsServer`)
    (`AdvancedFriendsLibrary.SendSessionInviteToFriend` (`GameplayStatics.GetPlayerController` 0) FriendUniqueNetId)))