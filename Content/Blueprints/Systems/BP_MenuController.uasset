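; BP_MenuController is the player controller for the menus, owning the menu widgets and handling session invites.
; On BeginPlay it creates and stores play, server, session, audio-settings and main menu widgets, showing and activating only the main menu.
; After a short delay it caches a DataHolderActor reference.
; Accepted invites go straight to JoinSession; the mouse-cursor and UI-only input nodes are unconnected.
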(event `self.ReceiveBeginPlay`
  (`|ExecutionSequence`
    (:`then_0`
      (bind _returnvalue (`|CreateWidget` "/Game/Widgets/WBP_PlayMenu.WBP_PlayMenu_C"))
      (set `self.PlayMenuRef` _returnvalue)
      (bind _returnvalue_2 (`|CreateWidget` "/Game/Widgets/WBP_CreateServer.WBP_CreateServer_C"))
      (set `self.CreateServerRef` _returnvalue_2)
      (bind _returnvalue_3 (`|CreateWidget` "/Game/Widgets/WBP_FindServers.WBP_FindServers_C"))
      (set `self.FindServersRef` _returnvalue_3)
      (bind _returnvalue_4 (`|CreateWidget` "/Game/Widgets/WBP_JoinSession.WBP_JoinSession_C"))
      (set `self.JoinSessionRef` _returnvalue_4)
      (bind _returnvalue_5 (`|CreateWidget` "/Game/Widgets/WBP_AudioSettings.WBP_AudioSettings_C"))
      (set `self.AudioSettingsRef` _returnvalue_5)
      (bind _returnvalue_6 (`|CreateWidget` "/Game/Widgets/WBP_MainMenu.WBP_MainMenu_C"))
      (bind _output_get (set `self.MainMenuRef` _returnvalue_6))
      (`UserWidget.AddToViewport` _output_get 0)
      (`CommonActivatableWidget.ActivateWidget` _output_get))
    (:`then_1`
      (`KismetSystemLibrary.Delay` 0.5)
      (bind _returnvalue_7 (`GameplayStatics.GetActorOfClass` "/Script/CoopProject.DataHolderActor"))
      (`/Engine/EditorBlueprintResources/StandardMacros.IsValid` _returnvalue_7
        (:`Is Valid`
          (set `self.DataHolderRef` _returnvalue_7))))))

(event `AdvancedFriendsInterface.OnSessionInviteAccepted`
  (params (PersonInvited :type "BPUniqueNetId Structure") (SearchResult :type "BlueprintSessionResult Structure (by ref)"))
  (`JoinSessionCallbackProxy.JoinSession` null SearchResult))

(fn `UserConstructionScript`)