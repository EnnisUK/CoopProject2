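; Player controller that handles the pause menu and traces for trigger actors in front of the player.
; On BeginPlay, the local controller creates the pause menu, starts a looping timer and binds Wi-Fi warning events, whose handlers are empty.
; LineTrace casts a debug-drawn ray along the camera's forward vector, storing or clearing the hit actor.
; High-ping icon and gamepad-detection logic are left disconnected.
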(event `EnhancedInput|/Game/Inputs/Actions/IA_PauseMenu`
  (params (ActionValue :type Boolean) (ElapsedSeconds :type "Float (double-precision)") (TriggeredSeconds :type "Float (double-precision)") (InputAction :type "InputAction Object Reference" :default "/Game/Inputs/Actions/IA_PauseMenu.IA_PauseMenu"))
  (:`Triggered`
    (if (`Widget.IsInViewport` (`self.PauseMenuRef`))
      (`Widget.RemoveFromParent` (`self.PauseMenuRef`))
      (else
        (`UserWidget.AddToViewport` (`self.PauseMenuRef`) 0)))))

(event `self.ReceiveBeginPlay`
  (if (`self.IsLocalPlayerController`)
    (`KismetSystemLibrary.K2_SetTimerDelegate` (`|CreateDelegate` :!event `LineTrace`) 0.1 true)
    (add `self.M_ShowWifi` (`|CreateDelegate` :!event `ShowWifiWarning`))
    (add `self.M_HideWifi` (`|CreateDelegate` :!event `HideWifiWarning`))
    (bind _returnvalue (`|CreateWidget` "/Game/Widgets/WBP_PauseMenu.WBP_PauseMenu_C"))
    (set `self.PauseMenuRef` _returnvalue)))

(event `ShowWifiWarning`)

(event `LineTrace`
  (bind _returnvalue (`GameplayStatics.GetPlayerCharacter` 0))
  (bind _returnvalue_2 (`self.K2_GetActorLocation` _returnvalue))
  (bind _outhit (`KismetSystemLibrary.LineTraceSingle` _returnvalue_2 (+ (* (`SceneComponent.GetForwardVector` (`self.GetComponentByClass` _returnvalue "/Script/Engine.CameraComponent")) 500.0) _returnvalue_2) "TraceTypeQuery2" true (`|MakeArray` (`GameplayStatics.GetPlayerCharacter` 0) :!type "Actor Object Reference") "ForDuration"))
  (bind (_bblockinghit _binitialoverlap _time _distance _location _impactpoint _normal _impactnormal _physmat _hitactor) (`GameplayStatics.BreakHitResult` _outhit))
  (if (`KismetMathLibrary.ClassIsChildOf` (`GameplayStatics.GetObjectClass` _hitactor))
    (bind _output_get (set `self.Hit Actor` _hitactor))
    (bind _astrigger_actor (cast `TriggerActor` _output_get))
    (set `self.As Trigger Actor 2` _astrigger_actor)
    (else
      (`/Engine/EditorBlueprintResources/StandardMacros.IsValid` null
        (:`Is Valid`
          (set `self.Hit Actor` null))))))

(event `HideWifiWarning`)

(event `self.ReceiveTick`
  (params (DeltaSeconds :type "Float (single-precision)")))

(fn `UserConstructionScript`)