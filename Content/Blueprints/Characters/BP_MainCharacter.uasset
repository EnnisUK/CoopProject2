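; BP_MainCharacter is the main character Blueprint, carrying a lantern and showing per-player lobby info.
; BeginPlay spawns BP_PlayerLantern on the mesh's LanternSocket and applies camera FOV and mouse sensitivity from the game instance.
; PlayerLobbyInfo's RepNotify updates and reveals the lobby widget, retrying on a short timer until the widget is valid.
; The lantern is destroyed along with the character.
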(event `self.ReceiveBeginPlay`
  (bind _returnvalue (`|SpawnActorFromClass` "/Game/Blueprints/Mechanics/BP_PlayerLantern.BP_PlayerLantern_C" (`SceneComponent.GetSocketTransform` (`self.Mesh`) "LanternSocket" "RTS_World") "Undefined" "MultiplyWithRoot" null null))
  (set `self.LanternRef` _returnvalue)
  (`self.K2_AttachToComponent` _returnvalue (`self.Mesh`) "LanternSocket" "SnapToTarget" "SnapToTarget" "SnapToTarget" true)
  (bind _asbp_afgi_main_instance (cast `/Game/Blueprints/Systems/BP_AFGI_MainInstance` (`GameplayStatics.GetGameInstance`)))
  (`CameraComponent.SetFieldOfView` (`self.M_Camera`) (`AFGI_MainInstance.M_FOV` _asbp_afgi_main_instance))
  (set `self.M_MouseSens` (`AFGI_MainInstance.M_MouseSens` _asbp_afgi_main_instance)))

(event `self.ReceiveDestroyed`
  (bind _lanternref (`self.LanternRef`))
  (`/Engine/EditorBlueprintResources/StandardMacros.IsValid` _lanternref
    (:`Is Valid`
      (`self.K2_DestroyActor` _lanternref))))

(fn `OnRep_PlayerLobbyInfo`
  (bind _returnvalue (`WidgetComponent.GetWidget` (`self.LobbyInfoWidget`)))
  (`KismetSystemLibrary.PrintString` "Hello")
  (`/Engine/EditorBlueprintResources/StandardMacros.IsValid` _returnvalue
    (:`Is Valid`
      (bind _aswbp_lobby_player_info (cast `/Game/Widgets/WBP_LobbyPlayerInfo` _returnvalue))
      (`/Game/Widgets/WBP_LobbyPlayerInfo.Update` _aswbp_lobby_player_info (`self.PlayerLobbyInfo`))
      (`SceneComponent.SetVisibility` (`self.LobbyInfoWidget`) true false))
    (:`Is Not Valid`
      (`KismetSystemLibrary.K2_SetTimer` null "OnRep_PlayerLobbyInfo" 0.1))))

(fn `UpdatePlayerLobbyInfo`
  (params (PlayerLobbyInfo :type "/Game/Blueprints/Lobby/S_PlayerLobbyInfo Structure"))
  (set `self.PlayerLobbyInfo` PlayerLobbyInfo))

(fn `UserConstructionScript`)